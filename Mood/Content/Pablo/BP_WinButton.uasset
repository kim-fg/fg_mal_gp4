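; BP_WinButton is an interactable button that ends the game through BP_FirstPersonGameMode.
; On Interact it calls the parent logic and plays a sound, then after a one-second delay stops its box blocking visibility traces and tints the button material green.
; A DoOnce then prints a debug message and calls GameFinished on the game mode, so the win fires only once.
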(event EventInteract
  (params (Player :type BP%20Player%20Character%20Object%20Reference))
  (|CallParentFunction 0)
  (Audio|PlaySoundatLocation "/Game/Mood/Sounds/SFX/Interaction/Interact_Cue.Interact_Cue" (Transformation|GetActorLocation) "0, 0, 0" 1.0 1.0 0.0 0 0 0 0)
  (Utilities|FlowControl|Delay 1.0)
  (Collision|SetCollisionResponsetoChannel (Variables|Default|GetBox) "ECC_Visibility" "ECR_Ignore")
  (Rendering|Material|SetVectorParameterValueonMaterials (Variables|Default|GetButton) "Holo Tint" "0.061108,0.578125,0.000000")
  (Utilities|FlowControl|DoOnce false
    (:Completed
      (Development|PrintString "Button Was Pressed")
      (bind _asbp_first_person_game_mode (Utilities|Casting|CastToBP_FirstPersonGameMode (Game|GetGameMode)))
      (Class|MoodGameMode|GameFinished _asbp_first_person_game_mode))))

(fn ConstructionScript)