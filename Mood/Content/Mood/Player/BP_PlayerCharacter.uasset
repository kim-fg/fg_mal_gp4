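; First-person player character Blueprint that lets the player interact with actors in view.
; The Interact input runs a short visibility line trace from the camera and sends InteractMessage to the hit actor.
; Tick repeats the trace, caching the hit actor and showing its info message, then hiding it and resetting a DoOnce when the target changes.
; The weapon slot's OnWeaponUsed event is bound but empty.
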(event OnWeaponUsed(WeaponSlotComponent)
  (params (Weapon :type Mood%20Weapon%20Component%20Object%20Reference)))

(event Input|EnhancedActionEvents|EnhancedInputActionIA_Interact
  (params (ActionValue :type Boolean) (ElapsedSeconds :type Float%20%28double-precision%29) (TriggeredSeconds :type Float%20%28double-precision%29) (InputAction :type Input%20Action%20Object%20Reference :default "/Game/FirstPerson/Input/Actions/IA_Interact.IA_Interact"))
  (bind _firstpersoncameracomponent (Variables|Default|GetFirstPersonCameraComponent))
  (bind _returnvalue (Transformation|GetWorldLocation _firstpersoncameracomponent))
  (:Started
    (bind _outhit (Collision|LineTraceByChannel _returnvalue (+ _returnvalue (* (Math|Vector|GetForwardVector _firstpersoncameracomponent) 2e+02)) "TraceTypeQuery1" false 0 "None"))
    (Class|BPMoodInteract|Interact(Message) (.HitActor (Collision|BreakHitResult _outhit)))))

(event EventTick
  (params (DeltaSeconds :type Float%20%28single-precision%29))
  (bind _firstpersoncameracomponent (Variables|Default|GetFirstPersonCameraComponent))
  (bind _returnvalue (Transformation|GetWorldLocation _firstpersoncameracomponent))
  (bind _outhit (Collision|LineTraceByChannel _returnvalue (+ _returnvalue (* (Math|Vector|GetForwardVector _firstpersoncameracomponent) 2e+02)) "TraceTypeQuery1" false 0 "None"))
  (Utilities|FlowControl|Sequence
    (:then_0
      (Utilities|FlowControl|DoOnce false :!label _label
        (:Completed
          _)))
    (:then_1
      (if (== (.HitActor (Collision|BreakHitResult _outhit)) (Variables|Default|GetInteractableActor))
        _
        (else
          (Class|BPMoodInteract|StopShowingInfo(Message) (Variables|Default|GetInteractableActor))
          (goto _label Reset)))))
  (bind _output_get (Variables|Default|SetInteractableActor (.HitActor (Collision|BreakHitResult _outhit))))
  (Class|BPMoodInteract|ShowInfo(Message) _output_get))

(fn ConstructionScript)