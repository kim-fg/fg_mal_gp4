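; Melee drone enemy character that adds attack animation, death effects and an execution material swap to its parent class.
; Weapon use from WeaponSlot triggers the attack montage.
; As an animation bug workaround, death hides the mesh, spawns a temporary BP_DroneSpawn with an explosion, silences the buzz and removes pawn collision and the hitbox.
; StartRagdoll is overridden empty, so the parent ragdoll never runs.
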(event OnDeath(Health)
  (params (DeadActor :type Actor%20Object%20Reference))
  (bind _mesh (Variables|Character|GetMesh))
  (bind _returnvalue (Transformation|GetWorldLocation _mesh))
  ;[1 1 1] Animation bug work around
  (Utilities|FlowControl|Sequence
    (:then_0
      (Rendering|SetVisibility (Variables|Character|GetMesh) false false)
      (Audio|Components|Audio|Stop (Variables|Default|GetDroneBuzz_Cue_0))
      (Rendering|Material|SetMaterial (Variables|Character|GetMesh) 0 "/Game/Art/DynamicMeshes/Melee_Enemy/Materials/MI_Enemydrone.MI_Enemydrone"))
    (:then_1
      (bind _returnvalue_2 (Game|SpawnActorfromClass "/Game/Mood/Enemy/BP_DroneSpawn.BP_DroneSpawn_C" (Math|Transform|MakeTransform _returnvalue "0, 0, 0" "1.000000,1.000000,1.000000") "Undefined" "MultiplyWithRoot" 0 0))
      (Niagara|SpawnSystematLocation "/Game/FirstPerson/Alessandro/vfx/Explosion_Small_NS.Explosion_Small_NS" _returnvalue)
      (Collision|SetCollisionResponsetoChannel (Variables|Default|GetCapsuleComponent) "ECC_Pawn" "ECR_Ignore")
      (Components|DestroyComponent (Variables|Default|GetHitBox))
      (Utilities|FlowControl|Delay 4.5)
      (Actor|DestroyActor _returnvalue_2))))

(event Custom|AttackAnimationCalled
  (params (Weapon :type Mood%20Weapon%20Component%20Object%20Reference))
  ;[1 1 1] Plays attacks animation
  (Development|PrintString "enemy attacked")
  (Animation|PlayAnimMontage "/Game/Art/DynamicMeshes/Melee_Enemy/Attack/Enemy_drone_attack_animation_v2_Montage.Enemy_drone_attack_animation_v2_Montage" 1.0 "None")
  (Utilities|FlowControl|Delay 3.0))

(event EventBeginPlay
  ;[1 1 1] Plays attacks animation
  (|CallParentFunction)
  (EventDispatchers|BindEventtoOnWeaponUsed (Variables|Default|GetWeaponSlot) (delegate Custom|AttackAnimationCalled)))

(event EventSetExecutionMaterial
  (Rendering|Material|SetMaterial (Variables|Character|GetMesh) 0 "/Game/Mood/Enemy/Execution_Materials/M_MeleeEnemyExecution.M_MeleeEnemyExecution"))

(fn ConstructionScript)

(fn StartRagdoll)