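; Base enemy character for Mood that runs a behavior tree on possession and writes a seen player to the blackboard.
; Melee variants play a drone buzz cue, and weapon use only prints a debug message.
; On death it stops AI logic, buzz and weapon trigger, spawns ammo for ranged variants, plays a destroyed sound, then ragdolls and despawns after a delay.
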(event OnDeath(Health)
  (params (DeadActor :type Actor%20Object%20Reference))
  ;[1 1 1] Death
  (Utilities|FlowControl|Sequence
    (:then_0
      (Audio|Components|Audio|Stop (Variables|Default|GetDroneBuzz_Cue))
      ;[1 1 1] Brain Death
      (AI|Logic|StopLogic (Variables|/Script/AIModule.AIController|GetBrainComponent (AI|GetAIController self)) "Death")
      (bind _returnvalue (Class|MoodEnemyCharacter|GetWeaponSlot))
      (Class|MoodWeaponSlotComponent|SetTriggerHeld _returnvalue false))
    (:then_1
      (Utilities|Casting|CastToBP_MoodRangedEnemyCharacter self)
      ;[1 1 1] Spawn ammo pickup
      (Game|SpawnActorfromClass "/Game/Mood/Weapons/BP_AmmoPickup.BP_AmmoPickup_C" (Transformation|GetActorTransform) "AdjustIfPossibleButAlwaysSpawn" "MultiplyWithRoot" 0 0))
    (:then_2
      (Audio|PlaySoundatLocation "/Game/Mood/Sounds/SFX/Enemies/Enemy_Destroyed_Cue.Enemy_Destroyed_Cue" (Transformation|GetActorLocation) "0, 0, 0" 1.0 1.0 0.0 0 0 0 0)
      ;[1 1 1] Ragdoll
      (CallFunction|StartRagdoll)
      (Utilities|FlowControl|Delay (Variables|Default|GetDespawn%20Delay))
      ;[1 1 1] Destruction
      (Actor|DestroyActor))))

(event Custom|OnPlayerSeen_Event
  (params (Player :type Mood%20Character%20Object%20Reference))
  ;[1 1 1] Sense Player
  (AI|Components|Blackboard|SetValueasObject (CallFunction|GetOwnedBlackboard) (Variables|Default|GetPlayer%20Key%20Name) Player))

(event Custom|OnWeaponUsed_Event
  (params (Weapon :type Mood%20Weapon%20Component%20Object%20Reference))
  (Development|PrintString "enemy attacked"))

(event EventBeginPlay
  (Utilities|FlowControl|Sequence
    (:then_0
      (EventDispatchers|BindEventtoOnWeaponUsed (Variables|Default|GetWeaponSlot) (delegate Custom|OnWeaponUsed_Event)))
    (:then_1
      (EventDispatchers|AssignOnPlayerSeen (delegate Custom|OnPlayerSeen_Event))
      (Utilities|Casting|CastToBP_MoodMeleeEnemyCharacter self)
      (Audio|Components|Audio|Play (Variables|Default|GetDroneBuzz_Cue) 0.0))))

(event EventPossessed
  (params (NewController :type Controller%20Object%20Reference))
  (bind _self self)
  (bind _returnvalue (AI|GetAIController _self))
  (Utilities|FlowControl|Sequence
    (:then_0
      ;[1 1 1] Start AI
      (Utilities|IsValid _returnvalue
        (:Is%20Valid
          (AI|RunBehaviorTree _returnvalue (Variables|Default|GetBehaviorTree)))
        (:Is%20Not%20Valid
          (Development|PrintString "ERROR: Mood enemy was spawned without AI Controller" false true "(R=1.000000,G=0.000000,B=0.000000,A=1.000000)"))))))

(fn ConstructionScript)

(fn GetOwnedBlackboard
  (return (AI|GetBlackboard (AI|GetAIController self))))

(fn StartRagdoll
  (Pawn|Components|CharacterMovement|DisableMovement (Variables|Character|GetCharacterMovement))
  (Components|DestroyComponent (Variables|Default|GetCapsuleComponent))
  (Components|Animation|SetAnimationMode (Variables|Character|GetMesh) "AnimationSingleNode" true)
  (Physics|SetSimulatePhysics (Variables|Character|GetMesh) true)
  (Collision|SetCollisionObjectType (Variables|Character|GetMesh) "ECC_PhysicsBody"))