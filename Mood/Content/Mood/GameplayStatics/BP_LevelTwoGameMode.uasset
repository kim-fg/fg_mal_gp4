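; Game mode for level two that ends the game once no BP_Portal actors remain in the level.
; Tick polls PortalCheckerLvl2, which searches for portals and crystals, updates CrystalsLeft and reports when the portals are gone.
; DoOnce gates make GameFinished fire a single time.
; A separate GetPortalsAndCrystals helper gathers both actor lists but is not called in this graph.
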(event EventBeginPlay
  (|CallParentFunction) ; This node is disabled and will not be called.\nDrag off pins to build functionality.
)

(event EventTick
  (params (DeltaSeconds :type Float%20%28single-precision%29))
  (|CallParentFunction DeltaSeconds)
  (bind _all_portals_destroyed (CallFunction|PortalCheckerLvl2 false))
  (if _all_portals_destroyed
    (Utilities|FlowControl|DoOnce false
      (:Completed
        (Class|MoodGameMode|GameFinished)))))

(fn ConstructionScript
  (|CallParentFunction))

(fn PortalCheckerLvl2
  (params (NewParam :type Boolean))
  ;[1 1 1] check if there are portals in the current level
  (bind _outactors (Actor|GetAllActorsOfClass "/Game/FirstPerson/Alessandro/bp/BP_Portal.BP_Portal_C"))
  (bind _outactors_2 (Actor|GetAllActorsOfClass "/Game/FirstPerson/Alessandro/bp/BP_Crystal.BP_Crystal_C"))
  (Variables|Default|SetCrystals%20Left (Class|KismetMathLibrary|ToInt64(Integer) (Utilities|Array|Length _outactors_2)))
  (bind _output_get (Variables|Default|SetPortals%20Destroyed (<= (Utilities|Array|Length _outactors) 0)))
  (if _output_get
    (Utilities|FlowControl|DoOnce false
      (:Completed
        (return (Variables|Default|GetPortals%20Destroyed))))))

(fn GetPortalsandCrystals
  (bind _outactors (Actor|GetAllActorsOfClass "/Game/FirstPerson/Alessandro/bp/BP_Portal.BP_Portal_C"))
  (bind _output_get (LocalVariables|SetNewLocalVar _outactors))
  (Variables|Default|SetOut%20Actors _output_get)
  (bind _outactors_2 (Actor|GetAllActorsOfClass "/Game/FirstPerson/Alessandro/bp/BP_Crystal.BP_Crystal_C"))
  (bind _output_get_2 (LocalVariables|SetNewLocalVar_0 _outactors_2))
  (Variables|Default|SetOut%20Actors_0 _output_get_2))