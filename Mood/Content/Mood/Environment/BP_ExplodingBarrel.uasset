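; BP_ExplodingBarrel is a barrel that explodes when its MoodHealth component reports death.
; On death it spawns a Niagara explosion, then sphere-overlaps Pawns using the RadialForce component's radius and applies ExplosionDamage to Characters that have a MoodHealthComponent.
; It then fires the radial impulse and destroys itself after a short delay.
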(event Custom|OnDeath
  (bind _cylinder (Variables|Default|GetCylinder))
  (bind _returnvalue (Transformation|GetWorldLocation _cylinder))
  (Niagara|SpawnSystematLocation "/Game/FirstPerson/Alessandro/vfx/Explosion_NS.Explosion_NS" _returnvalue)
  (bind _outactors (Collision|SphereOverlapActors _returnvalue (Variables|/Script/Engine.RadialForceComponent|GetRadius (Variables|Default|GetRadialForce)) (Utilities|Array|MakeArray "ObjectTypeQuery3") 0))
  (for _array_element _outactors
    (bind _ascharacter (Utilities|Casting|CastToCharacter _array_element))
    (Utilities|IsValid (Actor|GetComponentbyClass _ascharacter "/Script/Mood.MoodHealthComponent")
      (:Is%20Valid
        (Class|MoodHealthComponent|Hurt (Actor|GetComponentbyClass _ascharacter "/Script/Mood.MoodHealthComponent") (Variables|Default|GetExplosion%20damage)))))
  (Class|RadialForceComponent|FireImpulse (Variables|Default|GetRadialForce))
  (Utilities|FlowControl|Delay 0.2)
  (Actor|DestroyActor))

(event EventBeginPlay
  (EventDispatchers|BindEventtoOnDeath (Variables|Default|GetMoodHealth) (delegate Custom|OnDeath)))

(fn ConstructionScript)