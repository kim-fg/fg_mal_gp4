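; BP_DamageTickZone is an environment hazard that damages an overlapping actor with a MoodHealthComponent at regular intervals.
; Begin overlap stores that component and starts a looping one-second timer that calls Hurt on it.
; End overlap clears the target and timer only for the stored component.
; It tracks one target, so a new entrant replaces the stored component and timer handle without clearing the earlier timer.
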(event Custom|ApplyDamage
  (Class|MoodHealthComponent|Hurt (Variables|Default|GetTargetHealthComponent) 10))

(event Collision|EventActorBeginOverlap
  (params (OtherActor :type Actor%20Object%20Reference))
  (bind _returnvalue (Actor|GetComponentbyClass OtherActor "/Script/Mood.MoodHealthComponent"))
  (Utilities|IsValid _returnvalue
    (:Is%20Valid
      (Variables|Default|SetTargetHealthComponent _returnvalue)
      (bind _returnvalue_2 (Utilities|Time|SetTimerbyEvent (delegate Custom|ApplyDamage) 1.0 true))
      (Variables|Default|SetDamageTickTimer _returnvalue_2))))

(event Collision|EventActorEndOverlap
  (params (OtherActor :type Actor%20Object%20Reference))
  (bind _returnvalue (Actor|GetComponentbyClass OtherActor "/Script/Mood.MoodHealthComponent"))
  (Utilities|IsValid _returnvalue
    (:Is%20Valid
      (if (== _returnvalue (Variables|Default|GetTargetHealthComponent))
        (Variables|Default|SetTargetHealthComponent 0)
        (Utilities|Time|ClearandInvalidateTimerbyHandle (Variables|Default|GetDamageTickTimer))))))

(fn ConstructionScript)