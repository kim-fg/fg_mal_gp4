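; BP_MoodRangedEnemyCharacter is a ranged enemy character driven by the BT_MoodRangedEnemy behavior tree, which its AI controller starts on BeginPlay.
; PawnSensing stores any seen MoodCharacter as the player and writes it to the blackboard for the tree.
; On death from HealthComp, the mesh switches to physics simulation, ignores pawns and physics bodies, and the actor is destroyed after a despawn delay.
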(event OnDeath(healthComp)
  (Physics|SetSimulatePhysics (Variables|Character|GetMesh) true)
  (Collision|SetCollisionResponsetoChannel (Variables|Character|GetMesh) "ECC_Pawn" "ECR_Ignore")
  (Collision|SetCollisionResponsetoChannel (Variables|Character|GetMesh) "ECC_PhysicsBody" "ECR_Ignore")
  (Utilities|FlowControl|Delay (Variables|Default|GetdespawnDelay))
  (Actor|DestroyActor))

(event OnSeePawn(PawnSensing)
  (params (Pawn :type Pawn%20Object%20Reference))
  (bind _asmood_character (Utilities|Casting|CastToMoodCharacter Pawn))
  (Variables|Default|SetPlayer _asmood_character)
  (AI|Components|Blackboard|SetValueasObject (AI|GetBlackboard (AI|GetAIController self)) (Variables|Default|GetPlayerKeyName) (Variables|Default|GetPlayer)))

(event EventBeginPlay
  (AI|RunBehaviorTree (AI|GetAIController self) "/Game/Enemy/BehaviorTree/BT_MoodRangedEnemy.BT_MoodRangedEnemy"))

(fn ConstructionScript)